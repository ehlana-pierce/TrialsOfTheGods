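; BP_Button is a pressure plate that activates while the player character, BP_ThirdPersonCharacter_Xanthe, stands on it.
; Box overlap begin and end events, filtered by a cast to that character, set or clear IsActive and play a stone plate sound.
; SinkTimeline plays forward or in reverse to lerp the mesh's relative Z, sinking and raising the plate.
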(event `self.ReceiveBeginPlay`)

(event `self.Box.OnComponentBeginOverlap`
  (params (OverlappedComponent :type "PrimitiveComponent Object Reference") (OtherActor :type "Actor Object Reference") (OtherComp :type "PrimitiveComponent Object Reference") (OtherBodyIndex :type Integer) (bFromSweep :type Boolean) (SweepResult :type "HitResult Structure (by ref)"))
  (cast `/Game/ThirdPerson/Blueprints/BP_ThirdPersonCharacter_Xanthe` OtherActor)
  (`GameplayStatics.PlaySoundAtLocation` "/Game/TrialAssets/StonePressurePlate.StonePressurePlate" (`self.K2_GetActorLocation`) (struct) 1.0 1.0 0.0 null null null null)
  (set `self.IsActive` true)
  (bind (_direction _height) (`Timeline|SinkTimeline` :!label _label)
    (:`Update`
      (`SceneComponent.K2_SetRelativeLocation` (`self.StaticMesh`) (`KismetMathLibrary.MakeVector` 0.0 0.0 (`KismetMathLibrary.Lerp` 10.0 -10.0 _height)) false false))))

(event `self.Box.OnComponentEndOverlap`
  (params (OverlappedComponent :type "PrimitiveComponent Object Reference") (OtherActor :type "Actor Object Reference") (OtherComp :type "PrimitiveComponent Object Reference") (OtherBodyIndex :type Integer))
  (cast `/Game/ThirdPerson/Blueprints/BP_ThirdPersonCharacter_Xanthe` OtherActor)
  (`GameplayStatics.PlaySoundAtLocation` "/Game/TrialAssets/StonePressurePlate.StonePressurePlate" (`self.K2_GetActorLocation`) (struct) 1.0 1.0 0.0 null null null null)
  (set `self.IsActive` false)
  (goto _label :!via `Reverse`))

(fn `UserConstructionScript`)